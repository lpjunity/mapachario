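; Player character that hosts a grid-based inventory, with item pickup, interaction and point tallying.
; BeginPlay spawns grid render actors, waits briefly, initializes the pockets inventory, then creates inventory and window-layout widgets, layering windows on top.
; Input toggles the inventory with input context and mode, or sphere-traces forward to call GridInteractionInterface on the hit actor.
; Pickup delegates to the inventory widget; DropItem is an empty stub, with its spawn logic disconnected.
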(event `self.ReceiveBeginPlay`
  (`GridTextureGenerationSubsystem.SpawnIconGenerationRenderActor` (subsystem `GridTextureGenerationSubsystem`) (make `GridRenderTargetSpawnParams` "/GridInventory/Actors/BP_GridRenderTargetActor.BP_GridRenderTargetActor_C" (-500.0 0.0 50.0)))
  (`GridTextureGenerationSubsystem.SpawnGridRenderActors` (subsystem `GridTextureGenerationSubsystem`) (make `GridRenderTargetSpawnParams` "/GridInventory/Actors/BP_GridRenderTargetActor.BP_GridRenderTargetActor_C" (-500.0 -200.0 50.0)) 5 (0.0 -2000.0 0.0))
  (`KismetSystemLibrary.Delay` 0.1) ; We need this node because we want to give the GridTextureGenerationSubsystem \ntime to spawn rendering actors. \nIn your project, your probably want to have your own initialziation flow\nwhere you'll call InitInventory
  (`InventoryComponent.InitInventory` (`self.PlayerPocketsInventoryComponent`))
  (bind _returnvalue (`|CreateWidget` "/Game/04_BP/WBP_RacoonInventory.WBP_RacoonInventory_C" (`GameplayStatics.GetPlayerController` 0)))
  (set `self.PlayerInventoryWidget` _returnvalue)
  (bind _returnvalue_2 (`|CreateWidget` "/GridInventory/Widgets/WBP_WindowsLayout.WBP_WindowsLayout_C" (`GameplayStatics.GetPlayerController` 0)))
  (bind _output_get (set `self.WindowsLayoutWidget` _returnvalue_2))
  (`UserWidget.AddToViewport` _output_get 1) ; Windows Layout should have bigger zOrder than inventory,\nso we draw windows over player inventory
)

(event `EnhancedInput|/Game/04_BP/IA_ToggleInventory`
  (params (ActionValue :type Boolean) (ElapsedSeconds :type "Float (double-precision)") (TriggeredSeconds :type "Float (double-precision)") (InputAction :type "InputAction Object Reference" :default "/Game/04_BP/IA_ToggleInventory.IA_ToggleInventory"))
  (:`Completed`
    (`KismetSystemLibrary.PrintString` "I pressed")
    (`self.ToggleInventoryWidget`)))

(event `ToggleInventoryWidget`
  (bind _returnvalue (`GameplayStatics.GetPlayerController` 0))
  (bind _returnvalue_2 (`GameplayStatics.GetPlayerController` 0))
  (bind _playerinventorywidget (`self.PlayerInventoryWidget`))
  (if (`self.IsInventoryVisible`)
    (`Widget.RemoveFromParent` _playerinventorywidget)
    (`GridWindowsLayoutWidget.ClearLayout` (`self.WindowsLayoutWidget`))
    (`self.AddMainInputContext`)
    (set `PlayerController.bShowMouseCursor` true _returnvalue)
    (`WidgetBlueprintLibrary.SetInputMode_GameOnly` _returnvalue)
    (set `self.IsInventoryVisible` false)
    (else
      (`UserWidget.AddToViewport` _playerinventorywidget 0)
      (`self.RemoveMainInputContext`)
      (set `PlayerController.bShowMouseCursor` true _returnvalue_2)
      (`WidgetBlueprintLibrary.SetInputMode_GameAndUIEx` _returnvalue_2 null "DoNotLock" false)
      (set `self.IsInventoryVisible` true))))

(event `EnhancedInput|/Game/04_BP/IA_Interact`
  (params (ActionValue :type Boolean) (ElapsedSeconds :type "Float (double-precision)") (TriggeredSeconds :type "Float (double-precision)") (InputAction :type "InputAction Object Reference" :default "/Game/04_BP/IA_Interact.IA_Interact"))
  (bind _mesh (`self.Mesh`))
  (bind _returnvalue (+ (`SceneComponent.K2_GetComponentLocation` _mesh) (0.0 0.0 100.0)))
  (:`Completed`
    (`KismetSystemLibrary.PrintString` "E pressed")
    (bind (_outhit _returnvalue_2) (`KismetSystemLibrary.SphereTraceSingle` :`Start` _returnvalue :`End` (+ _returnvalue (* (`SceneComponent.GetForwardVector` _mesh) (`self.Distance`))) :`Radius` 100.0 :`TraceChannel` "TraceTypeQuery1" :`DrawDebugType` "ForDuration"))
    (if _returnvalue_2
      (bind (_bblockinghit _binitialoverlap _time _distance _location _impactpoint _normal _impactnormal _physmat _hitactor) (`GameplayStatics.BreakHitResult` _outhit))
      (if (`KismetSystemLibrary.DoesImplementInterface` _hitactor "/Script/GridInventory.GridInteractionInterface")
        (message `GridInteractionInterface.TryInteract` _hitactor self)))))

(event `GridCharacterInterface.DropItem`
  (params (InItem :type "GridItem Object Reference")))

(event `CountItemsPoints`
  (for _array_element (`Inventory.GetAllItems` (`InventoryComponent.GetInventory` (`self.PlayerPocketsInventoryComponent`)))
    (bind _asbp_point_item (cast `/Game/04_BP/Items/BP_PointItem` _array_element))
    (set `self.TotalPoints` (+ (`/Game/04_BP/Items/BP_PointItem.Points` _asbp_point_item) (`self.TotalPoints`))))
  (`KismetSystemLibrary.PrintString` (`KismetStringLibrary.Conv_DoubleToString` (`self.TotalPoints`))))

(fn `GetGridWindowsLayoutWidget`
  (returns (ReturnValue :type "GridWindowsLayoutWidget Object Reference"))
  (return (`self.WindowsLayoutWidget`)))

(fn `TryPickupItem`
  (params (Item :type "GridItem Object Reference"))
  (returns (`Was Pickedup` :type Boolean))
  (bind _success (`/Game/04_BP/WBP_RacoonInventory.TryEquipItemInAnyAvailableSlotOrInventory` (`self.PlayerInventoryWidget`) Item))
  (return _success))

(fn `UserConstructionScript`)