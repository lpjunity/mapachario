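; BP_House is a house that detects the raccoon player nearby and ends the game in defeat if they linger too long.
; Overlap with NoiseDetectionArea toggles the WBP_NoiseBar widget and sets a proximity flag that Tick uses to play or reverse a detection timeline.
; That timeline fills the noise bar, switching on the lights past a danger threshold.
; At the detection limit, a second timeline swings the door open before BP_TopDownGameMode ends the game.
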(event `self.ReceiveBeginPlay`
  (bind _dangerpercentage (`self.DangerPercentage`))
  (bind _aswbp_noise_bar (cast `/Game/04_BP/WBP_NoiseBar` (`WidgetComponent.GetUserWidgetObject` (`self.NoiseBar`))))
  (bind _output_get (set `self.NoiseWBP` _aswbp_noise_bar))
  (bind _output_get_2 (set `/Game/04_BP/WBP_NoiseBar.MaxNoisePercentage` (`self.TimeToBeDetected`) _output_get))
  (set `self.TimeToTurnOnLights` (* _output_get_2 _dangerpercentage))
  (set `/Game/04_BP/WBP_NoiseBar.AlarmPercentage` _dangerpercentage _output_get))

(event `self.ReceiveTick`
  (params (DeltaSeconds :type "Float (single-precision)"))
  (if (`self.IsRacoonInProximity`)
    (bind (_direction _time) (`Timeline|TimeToBeDetect` :!label _label)
      (:`Update`
        (bind _output_get (set `self.TimerToDetect` _time))
        (bind _output_get_2 (set `/Game/04_BP/WBP_NoiseBar.NoisePercentage` _output_get (`self.NoiseWBP`)))
        (`|ExecutionSequence`
          (:`then_0`
            (if (>= _output_get_2 (`self.TimeToTurnOnLights`))
              (`self.EnableLights`)
              (else
                (`self.DisableLights`))))
          (:`then_1`
            (if (>= _output_get_2 (`self.TimeToBeDetected`))
              (`self.OpenDoor`)
              (`KismetSystemLibrary.Delay` 1.0)
              (bind _asbp_top_down_game_mode (cast `/Game/01_Core/BP_TopDownGameMode` (`GameplayStatics.GetGameMode`)))
              (`/Game/01_Core/BP_TopDownGameMode.EndGame` _asbp_top_down_game_mode "You lose!" "You got too greedy today!"))))))
    (else
      (goto _label :!via `Reverse`))))

(event `self.NoiseDetectionArea.OnComponentBeginOverlap`
  (params (OverlappedComponent :type "PrimitiveComponent Object Reference") (OtherActor :type "Actor Object Reference") (OtherComp :type "PrimitiveComponent Object Reference") (OtherBodyIndex :type Integer) (bFromSweep :type Boolean) (SweepResult :type "HitResult Structure (by ref)"))
  (bind _asbp_character (cast `/Game/04_BP/BP_Character` OtherActor))
  (set `self.Racoon` _asbp_character)
  (`KismetSystemLibrary.PrintString` "Detecting raccon")
  (bind _output_get (set `self.IsRacoonInProximity` true))
  (`/Game/04_BP/WBP_NoiseBar.ToggleBar` (`self.NoiseWBP`) _output_get))

(event `self.NoiseDetectionArea.OnComponentEndOverlap`
  (params (OverlappedComponent :type "PrimitiveComponent Object Reference") (OtherActor :type "Actor Object Reference") (OtherComp :type "PrimitiveComponent Object Reference") (OtherBodyIndex :type Integer))
  (if (== OtherActor (`self.Racoon`))
    (set `self.Racoon` null)
    (`KismetSystemLibrary.PrintString` "Stop detecting racoon")
    (bind _output_get (set `self.IsRacoonInProximity` false))
    (`/Game/04_BP/WBP_NoiseBar.ToggleBar` (`self.NoiseWBP`) _output_get)))

(event `EnableLights`
  (`SceneComponent.SetVisibility` (`self.Lights`) true true))

(event `DisableLights`
  (`SceneComponent.SetVisibility` (`self.Lights`) false true))

(event `OpenDoor`
  (bind _door (`self.Door`))
  (bind (_direction _openingdoor) (`Timeline|TL_OpenDoor`)
    (:`Update`
      (`SceneComponent.K2_SetRelativeRotation` _door (`KismetMathLibrary.RLerp` (`KismetMathLibrary.Conv_VectorToRotator` (`SceneComponent.RelativeLocation` _door)) (struct :`Yaw` -80.0) _openingdoor) false false))))

(fn `UserConstructionScript`)