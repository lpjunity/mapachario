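; Interactable stash actor that holds a grid inventory of random items and lets the player move items to and from it.
; On BeginPlay, after a short delay for GridTextureGenerationSubsystem to spawn rendering actors, it initializes StashInventory and adds BP_PointItems built from random PossibleItems table rows.
; TryInteract puts a stash layout widget into the character's inventory widget's dynamic slot and toggles that screen.
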(event `self.ReceiveBeginPlay`
  (bind _possibleitems (`self.PossibleItems`))
  ; To use inventory we simple need to create Inventory component, then we can populate it with data.
  ; For this example I've used IA_Stash and added items. Then we can init inventory in Begin Play
  (set `self.ItemNumber` (`KismetMathLibrary.RandomIntegerInRange` 0 3))
  (bind _outrownames (`DataTableFunctionLibrary.GetDataTableRowNames` _possibleitems))
  (`KismetSystemLibrary.Delay` 0.1) ; We need this node because we want to give the GridTextureGenerationSubsystem \ntime to spawn rendering actors. \nIn your project, your probably want to have your own initialziation flow\nwhere you'll call InitInventory
  (`InventoryComponent.InitInventory` (`self.StashInventory`))
  (for _ (range (+ (`self.ItemNumber`) 1))
    (bind _returnvalue (`|GetDataTableRow` _possibleitems (`|GetArrayItem` _outrownames (`KismetMathLibrary.RandomIntegerInRange` 0 (- (`KismetArrayLibrary.Array_Length` _outrownames) 1))))
      (:`then`
        (bind (_itemname _itemdescription _dimensions _icon _points) (break `/Game/04_BP/Items/S_ItemData` _returnvalue))
        (bind _returnvalue_2 (`|GenericCreateObject` :`Class` "/Game/04_BP/Items/BP_PointItem.BP_PointItem_C" :`Points` _points :`ItemName` _itemname :`ItemDescription` _itemdescription :`Dimensions` _dimensions :`Icon` _icon :`ItemMesh` null :`ItemSkeletalMesh` null :`ItemDoubleClickActionClass` null))
        (`GridItem.InitItem` _returnvalue_2)
        (`Inventory.TryAddItem` (`InventoryComponent.GetInventory` (`self.StashInventory`)) _returnvalue_2)))))

(fn `TryInteract`
  (params (InstigatorActor :type "Actor Object Reference"))
  (returns (ReturnValue :type Boolean))
  (locals (GridCharacter :type "/Game/04_BP/BP_Character Object Reference"))
  (bind _asbp_character (cast `/Game/04_BP/BP_Character` InstigatorActor)
    (:`then`
      (set `local.GridCharacter` _asbp_character)
      (bind _asplayer_controller (cast `PlayerController` (`Pawn.GetController` (`local.GridCharacter`))))
      (bind _returnvalue (`|CreateWidget` "/GridInventory/WBP_InventoryLayout.WBP_InventoryLayout_C" _asplayer_controller)) ; We create a WBP_InventoryLayout and init it\nwith our Inventory from StashInventory component
      (`InventoryLayoutWidget.InitLayout` _returnvalue (`InventoryComponent.GetInventory` (`self.StashInventory`)))
      (`/GridInventory/WBP_PlayerInventory.PutWidgetInDynamicSlot` (`/Game/04_BP/BP_Character.PlayerInventoryWidget` (`local.GridCharacter`)) _returnvalue "Stash" false) ; The inventory layout widget is placed in a dynamic slot,\nso you can see both your character's inventory and the stash from this actor.\nThis way, you can move items between them easily.
      (`/Game/04_BP/BP_Character.ToggleInventoryWidget` (`local.GridCharacter`))
      (return true))
    (:`CastFailed`
      (return false))))

(fn `UserConstructionScript`)